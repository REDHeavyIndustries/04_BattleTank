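; AMortar_BP is a player-controlled mortar Blueprint that passes aiming setup and firing to a TankAiming component.
; BeginPlay initialises that component with the TankTurret and TankBarrel.
; Azimuth input yaws the AzimuthGimbal, scaled by delta time, and the Fire press calls Fire on the component.
; Elevation input does nothing, as the SpringArm pitch logic is left disconnected.
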(event `self.ReceiveBeginPlay`
  (`TankAimingComponent.InitialiseAim` (`self.TankAiming`) (`self.TankTurret`) (`self.TankBarrel`)))

(event `InputAxis|AimElevation`
  (params (AxisValue :type "Float (single-precision)")))

(event `InputAxis|AimAzimuth`
  (params (AxisValue :type "Float (single-precision)"))
  (`SceneComponent.K2_AddLocalRotation` (`self.Azimuth Gimbal`) (`KismetMathLibrary.MakeRotator` 0.0 0.0 (* AxisValue (`GameplayStatics.GetWorldDeltaSeconds`) 100.0)) false false))

(event `InputAction|Fire`
  (params (Key :type "Key Structure"))
  (:`Pressed`
    (`TankAimingComponent.Fire` (`self.TankAiming`))))

(fn `UserConstructionScript`)